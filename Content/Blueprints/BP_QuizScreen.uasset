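; In-world quiz screen actor that shows questions fetched from the Groq API and takes answers through physical overlap boxes.
; On BeginPlay it caches its WBP_Screen widget, requests questions for the GameInstance's persistent topic, and refreshes the UI when they load.
; Boxes A–D trigger matching widget answers, using a DoOnce and shared timed input lock against repeats.
; Box C skips the lock check, which sits in unconnected nodes.
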(event `self.ReceiveBeginPlay`
  (`KismetSystemLibrary.Delay` 0.5)
  (bind _aswbp_screen (cast `/Game/UI/WBP_Screen` (`WidgetComponent.GetUserWidgetObject` (`self.Screen`))))
  (set `self.Screen Ref` _aswbp_screen)
  (bind _asquiz_game_instance (cast `QuizGameInstance` (`GameplayStatics.GetGameInstance`))
    (:`then`
      ; Pobieranie pytań od API Groq
      (`QuizGameInstance.FetchQuestionsFromGroq` _asquiz_game_instance (`QuizGameInstance.PersistentTopic` _asquiz_game_instance) 15)
      (`KismetSystemLibrary.PrintString` "fetched")
      (add `QuizGameInstance.OnQuestionsLoaded` _asquiz_game_instance (delegate `OnQuestionsLoaded_Event`)))
    (:`CastFailed`
      (`KismetSystemLibrary.PrintString` "cast failed"))))

(event `OnQuestionsLoaded_Event`
  ; Załadowanie pytań do widgetu po udanym pobraniu od API
  (`/Game/UI/WBP_Screen.Update UI` (`self.Screen Ref`))
  (`KismetSystemLibrary.PrintString` "updating ui"))

(event `self.Box_answerA.OnComponentBeginOverlap`
  (params (OverlappedComponent :type "PrimitiveComponent Object Reference") (OtherActor :type "Actor Object Reference") (OtherComp :type "PrimitiveComponent Object Reference") (OtherBodyIndex :type Integer) (bFromSweep :type Boolean) (SweepResult :type "HitResult Structure (by ref)"))
  ; Fizyczna aktywacja odpowiedzi A
  (if (not (`self.bIsInputLocked`))
    (`/Engine/EditorBlueprintResources/StandardMacros.DoOnce` false :!label _label
      (:`Completed`
        (set `self.bIsInputLocked` true)
        (`/Game/UI/WBP_Screen.Trigger AnswerA` (`self.Screen Ref`))
        (`KismetSystemLibrary.Delay` 3.0)
        (set `self.bIsInputLocked` false)
        (goto _label :!via `Reset`)))))

(event `self.Box_answerB.OnComponentBeginOverlap`
  (params (OverlappedComponent :type "PrimitiveComponent Object Reference") (OtherActor :type "Actor Object Reference") (OtherComp :type "PrimitiveComponent Object Reference") (OtherBodyIndex :type Integer) (bFromSweep :type Boolean) (SweepResult :type "HitResult Structure (by ref)"))
  ; Fizyczna aktywacja odpowiedzi B
  (if (not (`self.bIsInputLocked`))
    (`/Engine/EditorBlueprintResources/StandardMacros.DoOnce` false :!label _label_2
      (:`Completed`
        (set `self.bIsInputLocked` true)
        (`/Game/UI/WBP_Screen.Trigger AnswerB` (`self.Screen Ref`))
        (`KismetSystemLibrary.Delay` 3.0)
        (set `self.bIsInputLocked` false)
        (goto _label_2 :!via `Reset`)))))

(event `self.Box_answerC.OnComponentBeginOverlap`
  (params (OverlappedComponent :type "PrimitiveComponent Object Reference") (OtherActor :type "Actor Object Reference") (OtherComp :type "PrimitiveComponent Object Reference") (OtherBodyIndex :type Integer) (bFromSweep :type Boolean) (SweepResult :type "HitResult Structure (by ref)"))
  ; Fizyczna aktywacja odpowiedzi C
  (`/Engine/EditorBlueprintResources/StandardMacros.DoOnce` false :!label _label_3
    (:`Completed`
      (set `self.bIsInputLocked` true)
      (`/Game/UI/WBP_Screen.Trigger AnswerC` (`self.Screen Ref`))
      (`KismetSystemLibrary.Delay` 3.0)
      (set `self.bIsInputLocked` false)
      (goto _label_3 :!via `Reset`))))

(event `self.Box_answerD.OnComponentBeginOverlap`
  (params (OverlappedComponent :type "PrimitiveComponent Object Reference") (OtherActor :type "Actor Object Reference") (OtherComp :type "PrimitiveComponent Object Reference") (OtherBodyIndex :type Integer) (bFromSweep :type Boolean) (SweepResult :type "HitResult Structure (by ref)"))
  ; Fizyczna aktywacja odpowiedzi D
  (if (not (`self.bIsInputLocked`))
    (`/Engine/EditorBlueprintResources/StandardMacros.DoOnce` false :!label _label_4
      (:`Completed`
        (set `self.bIsInputLocked` true)
        (`/Game/UI/WBP_Screen.Trigger AnswerD` (`self.Screen Ref`))
        (`KismetSystemLibrary.Delay` 3.0)
        (set `self.bIsInputLocked` false)
        (goto _label_4 :!via `Reset`)))))

(fn `UpdateScreen`
  (`KismetSystemLibrary.PrintString` "questions loaded"))

(fn `UserConstructionScript`)