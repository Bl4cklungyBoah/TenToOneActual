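; Actor that pulls throwable objects toward itself while a sphere wanders around a movement area.
; Collision overlaps track actors tagged "throwObject", and Tick applies force to their static mesh roots toward the actor's origin, growing with distance.
; On BeginPlay the sphere lowers, stores its start position, then a self-calling event repeatedly moves it to a random point in MovementArea's bounds and back.
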(event `self.collision.OnComponentBeginOverlap`
  (params (OverlappedComponent :type "PrimitiveComponent Object Reference") (OtherActor :type "Actor Object Reference") (OtherComp :type "PrimitiveComponent Object Reference") (OtherBodyIndex :type Integer) (bFromSweep :type Boolean) (SweepResult :type "HitResult Structure (by ref)"))
  ; podczas kolizji dodaje do listy jesli ma dobry tag
  (if (`self.ActorHasTag` OtherActor "throwObject")
    (`KismetArrayLibrary.Array_Add` (`self.targetsInRange`) OtherActor)))

(event `self.collision.OnComponentEndOverlap`
  (params (OverlappedComponent :type "PrimitiveComponent Object Reference") (OtherActor :type "Actor Object Reference") (OtherComp :type "PrimitiveComponent Object Reference") (OtherBodyIndex :type Integer))
  ; Usuwa element z listy gdy wychodzi z kolizji
  (if (`self.ActorHasTag` OtherActor "throwObject")
    (`KismetArrayLibrary.Array_RemoveItem` (`self.targetsInRange`) OtherActor)))

(event `self.ReceiveTick`
  (params (DeltaSeconds :type "Float (single-precision)"))
  (bind _returnvalue (`self.K2_GetActorLocation`))
  ; Przyciaganie elementow bedacyh w liscie
  (for _array_element (`self.targetsInRange`)
    (bind _asstatic_mesh_component (cast `StaticMeshComponent` (`Actor.RootComponent` _array_element)))
    (bind _returnvalue_2 (`self.K2_GetActorLocation` _array_element))
    (`PrimitiveComponent.AddForce` _asstatic_mesh_component (* (* (`KismetMathLibrary.Conv_RotatorToVector` (`KismetMathLibrary.FindLookAtRotation` _returnvalue_2 _returnvalue)) (`KismetMathLibrary.VSize` (- _returnvalue _returnvalue_2))) 50.0) "None" false)))

(event `self.ReceiveBeginPlay`
  (bind _returnvalue_location (`KismetMathLibrary.BreakTransform` (`SceneComponent.GetRelativeTransform` (`self.Sphere`))))
  (bind _returnvalue (`SceneComponent.GetRelativeTransform` (`self.Sphere`)))
  ; obnizenie obiektu na start
  (`KismetSystemLibrary.MoveComponentTo` (`self.Sphere`) (`KismetMathLibrary.MakeVector` (.x (.location _returnvalue)) (.y (.location _returnvalue)) (+ (.z (.location _returnvalue)) -150.0)) (struct) false false 1.0)
  (set `self.startPos` _returnvalue_location)
  (`KismetSystemLibrary.Delay` 1.0)
  (`self.CustomEvent`))

(event `CustomEvent`
  (bind (_origin _boxextent) (`KismetSystemLibrary.GetComponentBounds` (`self.Movement Area`)))
  ; Ruszanie sie obiektu do losowego miejsca i powrot na start
  (`KismetSystemLibrary.MoveComponentTo` (`self.Sphere`) (`KismetMathLibrary.InverseTransformLocation` (`self.GetTransform`) (`KismetMathLibrary.RandomPointInBoundingBox` _origin _boxextent)) (struct) false false 2.5)
  (`KismetSystemLibrary.Delay` 0.4)
  (`KismetSystemLibrary.MoveComponentTo` (`self.Sphere`) (`self.startPos`) (struct) false false 2.0)
  (`KismetSystemLibrary.Delay` 1.0)
  (`self.CustomEvent`))

(fn `UserConstructionScript`)