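; Moving wall actor whose Cube drifts endlessly between random points inside MovementBounds while changing size.
; A self-calling custom event runs timed MoveComponentTo moves with random pauses, insetting targets by the cube's scale.
; Each new move rerolls X and Z scale rates, which Tick applies per frame during movement, overriding them at size limits.
; The start position is stored on BeginPlay but not used.
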(event `self.ReceiveBeginPlay`
  ; Pozycja startowa
  (set `self.StartPosition` (`self.K2_GetActorLocation`))
  (`self.CustomEvent`))

(event `CustomEvent`
  (bind (_origin _boxextent) (`KismetSystemLibrary.GetComponentBounds` (`self.MovementBounds`)))
  ; Idzie do losowego punktu w MovementBounds
  (set `self.bIsFlying` true)
  (`KismetSystemLibrary.MoveComponentTo` (`self.Cube`) (`KismetMathLibrary.InverseTransformLocation` (`self.GetTransform`) (`KismetMathLibrary.RandomPointInBoundingBox` _origin (- _boxextent (* (`SceneComponent.RelativeScale3D` (`self.Cube`)) 50.0)))) (struct) false false (`KismetMathLibrary.RandomFloatInRange` 1.0 2.0))
  (set `self.bIsFlying` false)
  (`KismetSystemLibrary.Delay` (`KismetMathLibrary.RandomFloatInRange` 0.5 1.0))
  (`self.CustomEvent`)
  (set `self.ScaleX` (`KismetMathLibrary.RandomFloatInRange` -0.01 0.01))
  (set `self.ScaleZ` (`KismetMathLibrary.RandomFloatInRange` -0.01 0.01)))

(event `self.ReceiveTick`
  (params (DeltaSeconds :type "Float (single-precision)"))
  (bind _cube (`self.Cube`))
  (bind (_returnvalue_x _returnvalue_y _returnvalue_z) (`KismetMathLibrary.BreakVector` (`SceneComponent.K2_GetComponentScale` _cube)))
  ; zmiana sklai w czasie
  (if (`self.bIsFlying`)
    (if (< _returnvalue_x 7.0)
      (set `self.ScaleX` 0.01)
      (elif (> _returnvalue_x 11.0)
        (set `self.ScaleX` -0.01)))
    (if (< _returnvalue_z 3.0)
      (set `self.ScaleZ` 0.01)
      (elif (> _returnvalue_z 7.0)
        (set `self.ScaleZ` -0.01)))
    (`SceneComponent.SetWorldScale3D` _cube (`KismetMathLibrary.MakeVector` (+ _returnvalue_x (`self.ScaleX`)) _returnvalue_y (+ _returnvalue_z (`self.ScaleZ`))))))

(fn `UserConstructionScript`)