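; Keyboard-controlled character that walks, looks around, picks up and throws physics objects, and can switch to VR control.
; Enhanced Input drives movement and replaces the character with a spawned, possessed VRPawn on IA_ChangeCharacter.
; F toggles grabbing via a camera line trace and PhysicsHandle, whose target follows the camera on Tick.
; Holding IA_ThrowObject oscillates throw power between limits, and releasing it launches the held object along the camera's forward vector.
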(event `self.ReceiveBeginPlay`
  ; na start
  ;; załadowanie IMC klawiatura
  (bind _asplayer_controller (cast `PlayerController` (`self.GetController`)))
  (`EnhancedInputSubsystemInterface.AddMappingContext` (pcsubsystem `EnhancedInputLocalPlayerSubsystem` _asplayer_controller) "/Game/VRTemplate/Input/IMC_Keyboard.IMC_Keyboard" 0 (struct)))

(event `EnhancedInput|/Game/VRTemplate/Input/Actions/IA_Look`
  (params (ActionValue :type "Vector2D Structure") (ElapsedSeconds :type "Float (double-precision)") (TriggeredSeconds :type "Float (double-precision)") (InputAction :type "InputAction Object Reference" :default "/Game/VRTemplate/Input/Actions/IA_Look.IA_Look"))
  ; Ruszanie Kamera
  (:`Triggered`
    (`self.AddControllerYawInput` ActionValue_X)
    (`self.AddControllerPitchInput` (* ActionValue_Y -1.0))))

(event `EnhancedInput|/Game/VRTemplate/Input/Actions/IA_WASD`
  (params (ActionValue :type "Vector2D Structure") (ElapsedSeconds :type "Float (double-precision)") (TriggeredSeconds :type "Float (double-precision)") (InputAction :type "InputAction Object Reference" :default "/Game/VRTemplate/Input/Actions/IA_WASD.IA_WASD"))
  (bind (_returnvalue_roll _returnvalue_pitch _returnvalue_yaw) (`KismetMathLibrary.BreakRotator` (`self.GetControlRotation`)))
  (bind (_returnvalue_roll_2 _returnvalue_pitch_2 _returnvalue_yaw_2) (`KismetMathLibrary.BreakRotator` (`self.GetControlRotation`)))
  ; Chodzenie przod, tyl , lewo ,prawo
  (:`Triggered`
    (`self.AddMovementInput` (`KismetMathLibrary.GetRightVector` (`KismetMathLibrary.MakeRotator` _returnvalue_roll 0.0 _returnvalue_yaw)) ActionValue_X)
    (`self.AddMovementInput` (`KismetMathLibrary.GetForwardVector` (`KismetMathLibrary.MakeRotator` 0.0 0.0 _returnvalue_yaw_2)) ActionValue_Y)))

(event `EnhancedInput|/Game/VRTemplate/Input/Actions/IA_ChangeCharacter`
  (params (ActionValue :type Boolean) (ElapsedSeconds :type "Float (double-precision)") (TriggeredSeconds :type "Float (double-precision)") (InputAction :type "InputAction Object Reference" :default "/Game/VRTemplate/Input/Actions/IA_ChangeCharacter.IA_ChangeCharacter"))
  ; Zmiana aktora po kliknieciu/// Zmiana sterowania
  (:`Completed`
    (bind _output_get (set `self.WorldPos` (`KismetMathLibrary.Conv_VectorToTransform` (`self.K2_GetActorLocation`))))
    (`self.K2_DestroyActor`)
    (bind _returnvalue (`|SpawnActorFromClass` "/Game/VRTemplate/Blueprints/VRPawn.VRPawn_C" _output_get "Undefined" "MultiplyWithRoot" null null))
    (`Controller.Possess` (`GameplayStatics.GetPlayerController` 0) _returnvalue)))

(event `Key|F`
  (params (Key :type "Key Structure"))
  (bind _camera (`self.Camera`))
  (bind _returnvalue (`SceneComponent.K2_GetComponentLocation` _camera))
  ; Trzymanie przedmiotu
  (:`Pressed`
    (if (`self.IsHolding`)
      (`PhysicsHandleComponent.ReleaseComponent` (`self.PhysicsHandle`))
      (set `self.IsHolding` false)
      (else
        (bind (_outhit _returnvalue_2) (`KismetSystemLibrary.LineTraceSingle` _returnvalue (+ _returnvalue (* (`SceneComponent.GetForwardVector` _camera) 250.0)) "TraceTypeQuery1"))
        (if _returnvalue_2
          (bind (_bblockinghit _binitialoverlap _time _distance _location _impactpoint _normal _impactnormal _physmat _hitactor _hitcomponent) (`GameplayStatics.BreakHitResult` _outhit))
          (if (`SceneComponent.IsSimulatingPhysics` _hitcomponent "None")
            (set `self.HoldObject` _hitcomponent)
            (set `self.IsHolding` true)
            (`PhysicsHandleComponent.GrabComponentAtLocationWithRotation` (`self.PhysicsHandle`) _hitcomponent "None" (`SceneComponent.K2_GetComponentLocation` _hitcomponent) (`SceneComponent.K2_GetComponentRotation` _hitcomponent))))))))

(event `self.ReceiveTick`
  (params (DeltaSeconds :type "Float (single-precision)"))
  (bind _camera (`self.Camera`))
  ; Trzymanie przedmiotu
  ;; Odswiezanie lokazliazacji trzymanego przedmiotu
  (`PhysicsHandleComponent.SetTargetLocation` (`self.PhysicsHandle`) (+ (`SceneComponent.K2_GetComponentLocation` _camera) (* (`SceneComponent.GetForwardVector` _camera) 250.0))))

(event `EnhancedInput|/Game/VRTemplate/Input/Actions/IA_ThrowObject`
  (params (ActionValue :type Boolean) (ElapsedSeconds :type "Float (double-precision)") (TriggeredSeconds :type "Float (double-precision)") (InputAction :type "InputAction Object Reference" :default "/Game/VRTemplate/Input/Actions/IA_ThrowObject.IA_ThrowObject"))
  (bind _isholding (`self.IsHolding`))
  (bind _power (`self.Power`))
  ; rzut przedmiotem
  (:`Triggered`
    ;; zwiekszenie/zmniejszenie sily rzutu
    (if _isholding
      (if (`self.IncreasePower`)
        (bind _output_get (set `self.Power` (+ _power 10)))
        (set `self.IncreasePower` (>= (`self.MaxPower`) _output_get))
        (else
          (bind _output_get_2 (set `self.Power` (- _power 10)))
          (set `self.IncreasePower` (< _output_get_2 (`self.MinPower`)))))))
  (:`Started`
    ;; ustawienie parametrow sily
    (set `self.MaxPower` 2000)
    (set `self.MinPower` 0)
    (set `self.IncreasePower` true))
  (:`Completed`
    ;; rzucanie trzymanym przedmiotem
    (if _isholding
      (`PhysicsHandleComponent.ReleaseComponent` (`self.PhysicsHandle`))
      (set `self.IsHolding` false)
      (`PrimitiveComponent.AddImpulse` (`self.HoldObject`) (* (`SceneComponent.GetForwardVector` (`self.Camera`)) (`self.Power`)) "None" true)
      (set `self.Power` (`self.MinPower`)))))

(fn `UserConstructionScript`)